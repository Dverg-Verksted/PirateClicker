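; BP_PirateBase is a base pirate actor for Pirate Clicker that drives a health bar widget from its ability component.
; On BeginPlay it caches the WBP_PirateHealthBar from its WidgetHealth component and initializes it with the ability component's max health.
; The AbilitySystem's OnUpdateHealth event pushes each new health value to the cached bar, so the display updates without polling.
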(event `self.ReceiveBeginPlay`
  (bind _returnvalue (`self.GetAbilityComponent`))
  (`parent.ReceiveBeginPlay`)
  (bind _aswbp_pirate_health_bar (cast `/Game/PirateClicker/Core/UI/PiratesHealthBar/WBP_PirateHealthBar` (`WidgetComponent.GetWidget` (`self.Widget Health`))))
  (bind _output_get (set `self.As WBP Pirate Health Bar` _aswbp_pirate_health_bar))
  (`/Engine/EditorBlueprintResources/StandardMacros.IsValid` _output_get
    (:`Is Valid`
      (`/Engine/EditorBlueprintResources/StandardMacros.IsValid` _returnvalue
        (:`Is Valid`
          (`/Game/PirateClicker/Core/UI/PiratesHealthBar/WBP_PirateHealthBar.SetPirateHP` _output_get (`AbilitySystemComponent.GetMaxHealth` _returnvalue)))))))

(event `self.AbilitySystem.OnUpdateHealth`
  (params (NewHealth :type "Float (single-precision)"))
  (bind _as_wbp_pirate_health_bar (`self.As WBP Pirate Health Bar`))
  (`/Engine/EditorBlueprintResources/StandardMacros.IsValid` _as_wbp_pirate_health_bar
    (:`Is Valid`
      (`/Game/PirateClicker/Core/UI/PiratesHealthBar/WBP_PirateHealthBar.ChangePirateHP` _as_wbp_pirate_health_bar NewHealth))))

(fn `UserConstructionScript`)